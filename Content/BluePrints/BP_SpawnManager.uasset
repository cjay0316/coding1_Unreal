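; BP_SpawnManager runs enemy waves, starting the first shortly after BeginPlay.
; SpawnEnemies loops over every BP_SpwnPoint in the level and gives each a weighted random chance to spawn a BP_Enemy at its transform.
; NewWaveCheck, meant to be called by dying enemies, counts remaining BP_Enemy actors and respawns after a delay when at most one remains.
; Debug prints trace each step.
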(event `self.ReceiveBeginPlay`
  (`KismetSystemLibrary.PrintString` "Spawn Manager exists.") ; Tell the player that we exist
  (`KismetSystemLibrary.Delay` 1.0) ; Wait for some time
  (`self.Spawn Enemies`) ; Call the Soawn Enemies Event
)

(event `Spawn Enemies`
  (bind _outactors (`GameplayStatics.GetAllActorsOfClass` "/Game/BluePrints/BP_SpwnPoint.BP_SpwnPoint_C")) ; Get an array of all spawn points in the level
  (for _array_element _outactors
    (`KismetSystemLibrary.PrintString` (`KismetSystemLibrary.GetDisplayName` _array_element) true true (struct :`G` 1.0 :`B` 0.600114 :`A` 1.0) 10.0) ; print the name
    (if (`KismetMathLibrary.RandomBoolWithWeight` 0.8)
      (`|SpawnActorFromClass` "/Game/BluePrints/BP_Enemy.BP_Enemy_C" (`SceneComponent.K2_GetComponentToWorld` (`/Game/BluePrints/BP_SpwnPoint.DefaultSceneRoot` _array_element)) "Undefined" "MultiplyWithRoot" null null) ; Spawn Actor from class,\n BP_Enemy at the spawnpoints location
    ))
  (`KismetSystemLibrary.PrintString` "Finished with the For Each Loop for spawn enemies"))

(event `NewWaveCheck`
  (`KismetSystemLibrary.PrintString` "as that the last enemy?")
  (bind _outactors (`GameplayStatics.GetAllActorsOfClass` "/Game/BluePrints/BP_Enemy.BP_Enemy_C")) ; Get an array of all BP_Enemies in the level
  (bind _returnvalue (`KismetArrayLibrary.Array_Length` _outactors))
  (`KismetSystemLibrary.PrintString` (`KismetStringLibrary.Concat_StrStr` "There are" (`KismetStringLibrary.Conv_IntToString` _returnvalue) "enemies in the level."))
  (if (> _returnvalue 1)
    (`KismetSystemLibrary.PrintString` "You are not the last one.") ; Not time for new enemies yet
    (else
      (`KismetSystemLibrary.PrintString` "New Wave Encoming!" true true (struct :`R` 1.0 :`B` 0.03671 :`A` 1.0))
      (`KismetSystemLibrary.Delay` 3.0) ; Wait 3 seconds
      (`self.Spawn Enemies`) ; Spawn enemies again
    )))

(fn `UserConstructionScript`)