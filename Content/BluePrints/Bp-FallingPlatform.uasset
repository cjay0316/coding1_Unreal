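; Falling platform actor that drops after the player character steps into its trigger box, then returns to its starting spot.
; It runs a Ready, Activated, Falling, Resetting cycle with delays between stages, swapping the platform material at each.
; Falling enables physics simulation; resetting disables it and a timeline lerps the platform from its fallen transform back to the one saved at BeginPlay.
; An IsReady flag blocks retriggering until the return finishes.
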(event `self.ReceiveBeginPlay`
  ; Comment
  (set `self.Original_Transform` (`SceneComponent.K2_GetComponentToWorld` (`self.Platform`))))

(event `self.BoxTrigger.OnComponentBeginOverlap`
  (params (OverlappedComponent :type "PrimitiveComponent Object Reference") (OtherActor :type "Actor Object Reference") (OtherComp :type "PrimitiveComponent Object Reference") (OtherBodyIndex :type Integer) (bFromSweep :type Boolean) (SweepResult :type "HitResult Structure (by ref)"))
  ; Comment
  (`KismetSystemLibrary.PrintString` "Something ran into my trigger!")
  (if (`self.IsReady`)
    (cast `/Game/BluePrints/BP_Custom3rdpersonchar` OtherActor)
    (`self.Activated`)))

(event `Activated`
  ; Change color to active,
  (`KismetSystemLibrary.PrintString` "Activated!")
  (`PrimitiveComponent.SetMaterial` (`self.Platform`) 0 "/Game/Materials/PlatformMaterials/PlatformActivated.PlatformActivated")
  (set `self.IsReady` false)
  (`KismetSystemLibrary.Delay` (`self.ActiveDelayVariable`))
  (`self.Falling`))

(event `Falling`
  ; Comment
  (`KismetSystemLibrary.PrintString` "Falling!")
  (`PrimitiveComponent.SetMaterial` (`self.Platform`) 0 "/Game/Materials/PlatformMaterials/PlatformFalling.PlatformFalling")
  (`PrimitiveComponent.SetSimulatePhysics` (`self.Platform`) true) ; This turns gravity on  for the platform
  (`KismetSystemLibrary.Delay` (`self.FallDelayVariable`))
  (`self.Resetting`))

(event `Resetting`
  ; Comment
  (`KismetSystemLibrary.PrintString` "Resetting!")
  (`PrimitiveComponent.SetMaterial` (`self.Platform`) 0 "/Game/Materials/PlatformMaterials/PlatformReset.PlatformReset")
  (set `self.FallenTransform` (`SceneComponent.K2_GetComponentToWorld` (`self.Platform`)))
  (`PrimitiveComponent.SetSimulatePhysics` (`self.Platform`) false) ; This turns gravity off for the platform
  (bind (_direction _newtrack_0) (`Timeline|ReturnToStart`)
    (:`Update`
      (bind (_returnvalue_location _returnvalue_rotation) (`KismetMathLibrary.BreakTransform` (`KismetMathLibrary.TLerp` (`self.FallenTransform`) (`self.Original_Transform`) _newtrack_0)))
      (`SceneComponent.K2_SetWorldLocationAndRotation` (`self.Platform`) _returnvalue_location _returnvalue_rotation false false))
    (:`Finished`
      (set `self.IsReady` true) ; We are ready
      (`PrimitiveComponent.SetMaterial` (`self.Platform`) 0 "/Game/Materials/PlatformMaterials/PlatformReady.PlatformReady"))))

(fn `UserConstructionScript`)